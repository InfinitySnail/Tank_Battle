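; Player-controlled mortar Blueprint that handles camera orbit input and firing.
; On BeginPlay it hands its Barrel and Turret to the MortarAiming component, which also receives the Fire action.
; Azimuth input yaws AzimuthGimbal and altitude input pitches SpringArm, keeping the two camera axes separate.
; Controller axes are scaled by delta time for frame-rate independence, while mouse axes apply raw values.
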(event EventBeginPlay
  (Class|TankAimingComponent|Initialize (Variables|Default|GetMortarAiming) (Variables|Default|GetBarrel) (Variables|Default|GetTurret)))

(event Input|ActionEvents|InputActionFire
  (params (Key :type Key%20Structure))
  ;[1 1 1] Firing
  (:Pressed
    (Class|TankAimingComponent|Fire (Variables|Default|GetMortarAiming))))

(event Input|AxisEvents|InputAxisAimAzimuth
  (params (AxisValue :type Float%20%28single-precision%29))
  ;[1 1 1] Controller Camera Input
  (Transformation|AddLocalRotation (Variables|Default|GetAzimuth%20Gimbal) (Math|Rotator|MakeRotator 0.0 0.0 (* AxisValue (Utilities|Time|GetWorldDeltaSeconds) 1e+02)) false false))

(event Input|AxisEvents|InputAxisAimAltitude
  (params (AxisValue :type Float%20%28single-precision%29))
  (bind _spring_arm (Variables|Default|GetSpring%20Arm))
  ;[1 1 1] Controller Camera Input
  (Transformation|SetRelativeRotation _spring_arm (Math|Rotator|MakeRotator 0.0 (+ (.pitch (Variables|/Script/Engine.SceneComponent|GetRelativeRotation _spring_arm)) (* AxisValue (Utilities|Time|GetWorldDeltaSeconds) 1e+02)) 0.0) false false))

(event Input|AxisEvents|InputAxisAimAzimuth_Mouse
  (params (AxisValue :type Float%20%28single-precision%29))
  ;[1 1 1] Mouse Camera Input
  (Transformation|AddLocalRotation (Variables|Default|GetAzimuth%20Gimbal) (Math|Rotator|MakeRotator 0.0 0.0 AxisValue) false false))

(event Input|AxisEvents|InputAxisAimAltitude_Mouse
  (params (AxisValue :type Float%20%28single-precision%29))
  (bind _spring_arm (Variables|Default|GetSpring%20Arm))
  ;[1 1 1] Mouse Camera Input
  (Transformation|SetRelativeRotation _spring_arm (Math|Rotator|MakeRotator 0.0 (+ (.pitch (Variables|/Script/Engine.SceneComponent|GetRelativeRotation _spring_arm)) AxisValue) 0.0) false false))

(fn ConstructionScript)